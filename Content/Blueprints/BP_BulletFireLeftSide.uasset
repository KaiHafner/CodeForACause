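; Rotating left-side bullet-fire hazard that damages the third-person character with an invisible hitscan trace.
; A Timeline, played from Tick, yaws the root by its Rotation track scaled by ValueRot.
; Each Timeline update traces the Camera channel from Raycast1 along the actor's backward vector and damages the character on every hit.
; A DoOnce with no reset limits the hurt sound and debug print to the first hit.
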(event `self.ReceiveTick`
  (params (DeltaSeconds :type "Float (single-precision)"))
  (bind _raycast1 (`self.Raycast1`))
  (bind _returnvalue (`SceneComponent.K2_GetComponentLocation` _raycast1))
  (bind (_direction _rotation) (`Timeline|Timeline`)
    (:`Update`
      (`SceneComponent.K2_SetRelativeRotation` (`self.DefaultSceneRoot`) (`KismetMathLibrary.MakeRotator` 0.0 0.0 (* _rotation (`self.ValueRot`))) false false)
      (bind _outhit (`KismetSystemLibrary.LineTraceSingle` :`Start` _returnvalue :`End` (+ _returnvalue (* (`self.GetActorForwardVector` (`ActorComponent.GetOwner` _raycast1)) -100000.0)) :`TraceChannel` "TraceTypeQuery2" :`DrawTime` 0.1))
      (bind _asbp_third_person_character (cast `/Game/ThirdPerson/Blueprints/BP_ThirdPersonCharacter` (`.HitActor` (`GameplayStatics.BreakHitResult` _outhit))))
      (`GameplayStatics.ApplyDamage` _asbp_third_person_character 5.0)
      (`/Engine/EditorBlueprintResources/StandardMacros.DoOnce` false
        (:`Completed`
          (`GameplayStatics.PlaySound2D` "/Game/Audio/ouchShot.ouchShot" 1.0 1.0 0.0 null null)
          (`KismetSystemLibrary.PrintString` "Hello"))))))

(fn `UserConstructionScript`)