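; BP_Landmine is a landmine actor that detonates when an overlap with its Sphere component ends, rather than when it begins.
; On detonation it runs a small sphere overlap query at the Mine's location and damages any BP_ThirdPersonCharacter found.
; It then fires a RadialForce impulse, plays the landmine sound, spawns an explosion smoke emitter and destroys itself.
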(event `self.Sphere.OnComponentEndOverlap`
  (params (OverlappedComponent :type "PrimitiveComponent Object Reference") (OtherActor :type "Actor Object Reference") (OtherComp :type "PrimitiveComponent Object Reference") (OtherBodyIndex :type Integer))
  (bind _returnvalue (`SceneComponent.K2_GetComponentLocation` (`self.Mine`)))
  (bind _outactors (`KismetSystemLibrary.SphereOverlapActors` (`SceneComponent.K2_GetComponentLocation` (`self.Mine`)) 32.0 (`self.Object Types`)))
  (for _array_element _outactors
    (bind _asbp_third_person_character (cast `/Game/ThirdPerson/Blueprints/BP_ThirdPersonCharacter` _array_element))
    (`GameplayStatics.ApplyDamage` _asbp_third_person_character 100.0))
  (`RadialForceComponent.FireImpulse` (`self.RadialForce`))
  (`GameplayStatics.PlaySoundAtLocation` "/Game/Audio/Landmine.Landmine" _returnvalue (struct) 1.0 1.0 0.0 null null null null)
  (`GameplayStatics.SpawnEmitterAtLocation` "/Game/Realistic_Starter_VFX_Pack_Vol2/Particles/Explosion/P_Explosion_Smoke.P_Explosion_Smoke" _returnvalue)
  (`self.K2_DestroyActor`))

(fn `UserConstructionScript`)