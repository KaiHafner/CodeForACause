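; Ambient audio Blueprint that loops three battlefield-style sound layers: explosions, bullets and triple shots.
; Each audio component's OnAudioFinished event waits a short random delay within its own range, then calls a small function that replays that sound from the start.
; The layers repeat independently with varied gaps; the graph contains no initial trigger, only these replay chains.
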(event `self.ambientExplosion.OnAudioFinished`
  (`KismetSystemLibrary.Delay` (`KismetMathLibrary.RandomFloatInRange` 2.0 3.0))
  (`self.ambientExplosionFunc`))

(event `self.ambientBullets.OnAudioFinished`
  (`KismetSystemLibrary.Delay` (`KismetMathLibrary.RandomFloatInRange` 1.0 1.2))
  (`self.ambientBulletsFunc`))

(event `self.ambientTripleShot.OnAudioFinished`
  (`KismetSystemLibrary.Delay` (`KismetMathLibrary.RandomFloatInRange` 1.0 2.0))
  (`self.ambientTripleshotFunc`))

(fn `ambientBulletsFunc`
  (`AudioComponent.Play` (`self.ambientBullets`) 0.0))

(fn `ambientExplosionFunc`
  (`AudioComponent.Play` (`self.ambientExplosion`) 0.0))

(fn `ambientTripleshotFunc`
  (`AudioComponent.Play` (`self.ambientTripleShot`) 0.0))

(fn `UserConstructionScript`)